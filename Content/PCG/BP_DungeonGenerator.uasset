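; Procedural dungeon generator actor that grows a seeded layout of PCG rooms and tunnels at BeginPlay.
; It spawns a BP_RandomSpline room, then picks random door arrows and probes each with a scaled BP_CollisionValider.
; Blocked doors are dropped; clear ones get wall destroyers, a tunnel and a randomized room whose doors join the pool, until none remain.
; Delay loops await async steps; yaw quadrants orient spawn offsets.
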(event Custom|Generate%20First%20Room
  (bind _possibledoors (Variables|Default|GetPossibleDoors))
  (bind _returnvalue (Game|SpawnActorfromClass "/Game/PCG/BP_RandomSpline.BP_RandomSpline_C" (Math|Transform|MakeTransform (Transformation|GetWorldLocation (Variables|Default|GetDefaultSceneRoot)) "0, 0, 0" "1.000000,1.000000,1.000000") "AlwaysSpawn" "MultiplyWithRoot" 0 false (Variables|Default|GetRandom%20Seed) 32 false 5e+02 4e+03 4e+03 false true false 2e+03 0))
  (Class|PCGComponent|GenerateLocal (Variables|/Game/PCG/BP_RandomSpline.BP_RandomSpline_C|GetPCG _returnvalue) false)
  (Utilities|Array|Clear _possibledoors)
  (Utilities|Array|AppendArray _possibledoors (Components|GetChildrenComponents (Variables|/Game/PCG/BP_RandomSpline.BP_RandomSpline_C|GetArrows _returnvalue) false))
  (Utilities|Array|RemoveIndex _possibledoors)
  (Utilities|Array|RemoveIndex _possibledoors)
  (if (Variables|/Game/PCG/BP_RandomSpline.BP_RandomSpline_C|GetDoneGenerating _returnvalue) :!label _label
    (Development|PrintString "done" false)
    (bind _output_get (Variables|Default|SetChosen%20Index (Math|Random|RandomIntegerinRangefromStream (Variables|Default|GetStream) 0 4)))
    (bind _returnvalue_2 (Game|SpawnActorfromClass "/Game/PCG/BP_WallDestroyer.BP_WallDestroyer_C" (Math|Transform|MakeTransform (Transformation|GetWorldLocation (Utilities|Array|Get(acopy) _possibledoors _output_get)) (Math|Rotator|MakeRotator 0.0 0.0 (.yaw (Transformation|GetWorldRotation (Utilities|Array|Get(acopy) _possibledoors _output_get)))) "1.000000,1.000000,1.000000") "AlwaysSpawn" "MultiplyWithRoot" 0 0))
    (if (and (>= (.yaw (Transformation|GetWorldRotation (Utilities|Array|Get(acopy) _possibledoors _output_get))) -45.0) (<= (.yaw (Transformation|GetWorldRotation (Utilities|Array|Get(acopy) _possibledoors _output_get))) 45.0))
      (Transformation|AddActorWorldOffset _returnvalue_2 "-100.000000,-180.000000,-50.000000")
      (elif (and (>= (.yaw (Transformation|GetWorldRotation (Utilities|Array|Get(acopy) _possibledoors _output_get))) 135.0) (<= (.yaw (Transformation|GetWorldRotation (Utilities|Array|Get(acopy) _possibledoors _output_get))) 225.0))
        (Transformation|AddActorWorldOffset _returnvalue_2 "100.000000,180.000000,-50.000000")
        (elif (and (>= (.yaw (Transformation|GetWorldRotation (Utilities|Array|Get(acopy) _possibledoors _output_get))) 45.0) (<= (.yaw (Transformation|GetWorldRotation (Utilities|Array|Get(acopy) _possibledoors _output_get))) 135.0))
          (Transformation|AddActorWorldOffset _returnvalue_2 "180.000000,-100.000000,-50.000000")
          (else
            (Transformation|AddActorWorldOffset _returnvalue_2 "-180.000000,100.000000,-50.000000")))))
    (Variables|Default|SetFirst%20Room%20Done%20? true)
    (else
      (Utilities|FlowControl|Delay 0.05)
      (Development|PrintString "waiting" false)
      (goto _label))))

(event Custom|Generate%20Another%20Room
  (bind _possibledoors (Variables|Default|GetPossibleDoors))
  (bind _possibledoors_2 (Variables|Default|GetPossibleDoors))
  (bind _possibledoors_3 (Variables|Default|GetPossibleDoors))
  (bind _possibledoors_4 (Variables|Default|GetPossibleDoors))
  (bind _stream (Variables|Default|GetStream))
  (bind _stream_2 (Variables|Default|GetStream))
  (bind _returnvalue (Utilities|Array|Length _possibledoors_3))
  (bind _output_get (Variables|Default|SetChosen%20Index (Utilities|Array|LastIndex _possibledoors_2)))
  (bind _returnvalue_2 (Game|SpawnActorfromClass "/Game/PCG/BP_WallDestroyer.BP_WallDestroyer_C" (Math|Transform|MakeTransform (Transformation|GetWorldLocation (Utilities|Array|Get(acopy) _possibledoors_2 _output_get)) (Math|Rotator|MakeRotator 0.0 0.0 (.yaw (Transformation|GetWorldRotation (Utilities|Array|Get(acopy) _possibledoors_2 _output_get)))) "1.000000,1.000000,1.000000") "AlwaysSpawn" "MultiplyWithRoot" 0 0))
  (CallFunction|GetRotation (Utilities|Array|Get(acopy) _possibledoors_2 _output_get) _returnvalue_2 1e+02 -1e+02 -5e+01)
  (bind _returnvalue_3 (Game|SpawnActorfromClass "/Game/PCG/BP_RandomSpline.BP_RandomSpline_C" (Math|Transform|MakeTransform (Transformation|GetWorldLocation (Utilities|Array|Get(acopy) _possibledoors_2 _output_get)) (Math|Rotator|MakeRotator 0.0 0.0 (.yaw (Transformation|GetWorldRotation (Utilities|Array|Get(acopy) _possibledoors_2 _output_get)))) "1.000000,1.000000,1.000000") "AlwaysSpawn" "MultiplyWithRoot" 0 false (Math|Random|RandomIntegerinRangefromStream _stream_2 1000 9999) (Variables|Default|GetNumOfPoints) false (Variables|Default|GetDistanceBetween) (Math|Random|RandomFloatinRangefromStream _stream_2 1e+03 2.5e+03) (Math|Random|RandomFloatinRangefromStream _stream_2 2.5e+03 4e+03) false (Class|KismetMathLibrary|RandomBoolwithWeightfromStream _stream_2 0.5) (Class|KismetMathLibrary|RandomBoolwithWeightfromStream _stream_2 0.75) (Math|Random|RandomFloatinRangefromStream _stream_2 1e+03 2.5e+03) 0))
  (CallFunction|GetRotation (Utilities|Array|Get(acopy) _possibledoors_2 _output_get) _returnvalue_3 1e+02 0.0 0.0)
  (Class|PCGComponent|GenerateLocal (Variables|/Game/PCG/BP_RandomSpline.BP_RandomSpline_C|GetPCG _returnvalue_3) false)
  (if (Variables|/Game/PCG/BP_RandomSpline.BP_RandomSpline_C|GetDoneGenerating _returnvalue_3) :!label _label
    (Utilities|Array|RemoveIndex _possibledoors (Variables|Default|GetChosen%20Index))
    (Utilities|Array|AppendArray _possibledoors (Components|GetChildrenComponents (Variables|/Game/PCG/BP_RandomSpline.BP_RandomSpline_C|GetArrows _returnvalue_3) false))
    (for (_array_element _array_index) (Variables|Default|GetPossibleDoors)
      (if (not (Utilities|String|Contains (Utilities|GetDisplayName _array_element) "arrow"))
        (Utilities|Array|Add (Variables|Default|GetIndexes%20To%20Delete) _array_index)))
    (bind _arrayelement (Utilities|Array|ReverseforEachLoop (Variables|Default|GetIndexes%20To%20Delete))
      (:LoopBody
        (Utilities|Array|RemoveIndex (Variables|Default|GetPossibleDoors) _arrayelement))
      (:Completed
        (Utilities|Array|Clear (Variables|Default|GetIndexes%20To%20Delete))
        ;[1 1 1] Tunnel
        (if (!= _returnvalue 0) :!label _label_2
          (bind _output_get_2 (Variables|Default|SetChosen%20Index (Math|Random|RandomIntegerinRangefromStream (Variables|Default|GetStream) 0 (- _returnvalue 1))))
          (if (and (>= (.yaw (Transformation|GetWorldRotation (Utilities|Array|Get(acopy) _possibledoors_3 _output_get_2))) -45.0) (<= (.yaw (Transformation|GetWorldRotation (Utilities|Array|Get(acopy) _possibledoors_3 _output_get_2))) 45.0))
            (Variables|Default|SetOffset "150.000000,0.000000,0.000000")
            (elif (and (>= (.yaw (Transformation|GetWorldRotation (Utilities|Array|Get(acopy) _possibledoors_3 _output_get_2))) 135.0) (<= (.yaw (Transformation|GetWorldRotation (Utilities|Array|Get(acopy) _possibledoors_3 _output_get_2))) 225.0))
              (Variables|Default|SetOffset "-150.000000,0.000000,0.000000")
              (elif (and (>= (.yaw (Transformation|GetWorldRotation (Utilities|Array|Get(acopy) _possibledoors_3 _output_get_2))) 45.0) (<= (.yaw (Transformation|GetWorldRotation (Utilities|Array|Get(acopy) _possibledoors_3 _output_get_2))) 135.0))
                (Variables|Default|SetOffset "0.000000,150.000000,0.000000")
                (else
                  (Variables|Default|SetOffset "0.000000,-150.000000,0.000000")))))
          (Variables|Default|SetDistanceBetween (Math|Random|RandomFloatinRangefromStream _stream 2.5e+02 7.5e+02))
          (Variables|Default|SetNumOfPoints (Math|Random|RandomIntegerinRangefromStream _stream 8 64))
          (Variables|Default|SetScaleLengthOfValider (/ (* (/ (Variables|Default|GetNumOfPoints) 4) (Variables|Default|GetDistanceBetween)) 55.0))
          (bind _returnvalue_4 (Game|SpawnActorfromClass "/Game/PCG/BP_CollisionValider.BP_CollisionValider_C" (Math|Transform|MakeTransform (+ (Transformation|GetWorldLocation (Utilities|Array|Get(acopy) _possibledoors_3 _output_get_2)) (Variables|Default|GetOffset)) (Math|Rotator|MakeRotator 0.0 0.0 (.yaw (Transformation|GetWorldRotation (Utilities|Array|Get(acopy) _possibledoors_3 _output_get_2)))) (Math|Vector|MakeVector 1.0 (Variables|Default|GetScaleLengthOfValider) 1.0)) "Undefined" "MultiplyWithRoot" 0 (Variables|Default|GetOffset) 0))
          (Utilities|FlowControl|Delay 1.0)
          (if (Variables|/Game/PCG/BP_CollisionValider.BP_CollisionValider_C|GetDone _returnvalue_4) :!label _label_3
            (if (Variables|/Game/PCG/BP_CollisionValider.BP_CollisionValider_C|GetHit? _returnvalue_4)
              (Development|PrintString "YES")
              (Utilities|Array|RemoveIndex (Variables|Default|GetPossibleDoors) (Variables|Default|GetChosen%20Index))
              (Actor|DestroyActor _returnvalue_4)
              (goto _label_2)
              (else
                (Development|PrintString "NO")
                (Actor|DestroyActor _returnvalue_4)
                (bind _returnvalue_5 (Game|SpawnActorfromClass "/Game/PCG/BP_WallDestroyer.BP_WallDestroyer_C" (Math|Transform|MakeTransform (Transformation|GetWorldLocation (Utilities|Array|Get(acopy) (Variables|Default|GetPossibleDoors) (Variables|Default|GetChosen%20Index))) (Math|Rotator|MakeRotator 0.0 0.0 (.yaw (Transformation|GetWorldRotation (Utilities|Array|Get(acopy) (Variables|Default|GetPossibleDoors) (Variables|Default|GetChosen%20Index))))) "1.000000,1.000000,1.000000") "AlwaysSpawn" "MultiplyWithRoot" 0 0))
                (CallFunction|GetRotation (Utilities|Array|Get(acopy) (Variables|Default|GetPossibleDoors) (Variables|Default|GetChosen%20Index)) _returnvalue_5 1e+02 2e+02 -5e+01)
                (bind _returnvalue_6 (Game|SpawnActorfromClass "/Game/PCG/BP_Tunnel.BP_Tunnel_C" (Math|Transform|MakeTransform (Transformation|GetWorldLocation (Utilities|Array|Get(acopy) (Variables|Default|GetPossibleDoors) (Variables|Default|GetChosen%20Index))) (Math|Rotator|MakeRotator 0.0 0.0 (.yaw (Transformation|GetWorldRotation (Utilities|Array|Get(acopy) (Variables|Default|GetPossibleDoors) (Variables|Default|GetChosen%20Index))))) "1.000000,1.000000,1.000000") "AlwaysSpawn" "MultiplyWithRoot" 0 0))
                (PCG|Generate (Variables|/Game/PCG/BP_Tunnel.BP_Tunnel_C|GetPCGTunnel _returnvalue_6) false)
                (Transformation|SetWorldTransform (Variables|/Game/PCG/BP_Tunnel.BP_Tunnel_C|GetExit _returnvalue_6) (Math|Transform|MakeTransform (.location (Transformation|GetWorldTransform (Variables|/Game/PCG/BP_Tunnel.BP_Tunnel_C|GetExit _returnvalue_6))) (.rotation (Transformation|GetWorldTransform (Utilities|Array|Get(acopy) (Variables|Default|GetPossibleDoors) (Variables|Default|GetChosen%20Index)))) (.scale (Transformation|GetWorldTransform (Variables|/Game/PCG/BP_Tunnel.BP_Tunnel_C|GetExit _returnvalue_6)))) false false)
                (Utilities|Array|Add _possibledoors_4 (Variables|/Game/PCG/BP_Tunnel.BP_Tunnel_C|GetExit _returnvalue_6))
                (Utilities|Array|RemoveIndex _possibledoors_4 (Variables|Default|GetChosen%20Index))
                (Development|PrintString "done spawning")
                (CallFunction|GenerateAnotherRoom)))
            (else
              (Utilities|FlowControl|Delay 0.1)
              (goto _label_3)))
          (else
            (Development|PrintString "No exits")))))
    (else
      (Utilities|FlowControl|Delay 0.05)
      (goto _label))))

(event Custom|Generate%20Tunnel
  (bind _possibledoors (Variables|Default|GetPossibleDoors))
  (bind _possibledoors_2 (Variables|Default|GetPossibleDoors))
  (bind _stream (Variables|Default|GetStream))
  (bind _returnvalue (Utilities|Array|Length _possibledoors))
  (if (Variables|Default|GetFirst%20Room%20Done%20?) :!label _label
    ;[1 1 1] Tunnel
    (if (!= _returnvalue 0) :!label _label_2
      (bind _output_get (Variables|Default|SetChosen%20Index (Math|Random|RandomIntegerinRangefromStream (Variables|Default|GetStream) 0 (- _returnvalue 1))))
      (if (and (>= (.yaw (Transformation|GetWorldRotation (Utilities|Array|Get(acopy) _possibledoors _output_get))) -45.0) (<= (.yaw (Transformation|GetWorldRotation (Utilities|Array|Get(acopy) _possibledoors _output_get))) 45.0))
        (Variables|Default|SetOffset "150.000000,0.000000,0.000000")
        (elif (and (>= (.yaw (Transformation|GetWorldRotation (Utilities|Array|Get(acopy) _possibledoors _output_get))) 135.0) (<= (.yaw (Transformation|GetWorldRotation (Utilities|Array|Get(acopy) _possibledoors _output_get))) 225.0))
          (Variables|Default|SetOffset "-150.000000,0.000000,0.000000")
          (elif (and (>= (.yaw (Transformation|GetWorldRotation (Utilities|Array|Get(acopy) _possibledoors _output_get))) 45.0) (<= (.yaw (Transformation|GetWorldRotation (Utilities|Array|Get(acopy) _possibledoors _output_get))) 135.0))
            (Variables|Default|SetOffset "0.000000,150.000000,0.000000")
            (else
              (Variables|Default|SetOffset "0.000000,-150.000000,0.000000")))))
      (Variables|Default|SetDistanceBetween (Math|Random|RandomFloatinRangefromStream _stream 2.5e+02 7.5e+02))
      (Variables|Default|SetNumOfPoints (Math|Random|RandomIntegerinRangefromStream _stream 8 64))
      (Variables|Default|SetScaleLengthOfValider (/ (* (/ (Variables|Default|GetNumOfPoints) 4) (Variables|Default|GetDistanceBetween)) 55.0))
      (bind _returnvalue_2 (Game|SpawnActorfromClass "/Game/PCG/BP_CollisionValider.BP_CollisionValider_C" (Math|Transform|MakeTransform (+ (Transformation|GetWorldLocation (Utilities|Array|Get(acopy) _possibledoors _output_get)) (Variables|Default|GetOffset)) (Math|Rotator|MakeRotator 0.0 0.0 (.yaw (Transformation|GetWorldRotation (Utilities|Array|Get(acopy) _possibledoors _output_get)))) (Math|Vector|MakeVector 1.0 (Variables|Default|GetScaleLengthOfValider) 1.0)) "Undefined" "MultiplyWithRoot" 0 (Variables|Default|GetOffset) 0))
      (Utilities|FlowControl|Delay 1.0)
      (if (Variables|/Game/PCG/BP_CollisionValider.BP_CollisionValider_C|GetDone _returnvalue_2) :!label _label_3
        (if (Variables|/Game/PCG/BP_CollisionValider.BP_CollisionValider_C|GetHit? _returnvalue_2)
          (Development|PrintString "YES")
          (Utilities|Array|RemoveIndex (Variables|Default|GetPossibleDoors) (Variables|Default|GetChosen%20Index))
          (Actor|DestroyActor _returnvalue_2)
          (goto _label_2)
          (else
            (Development|PrintString "NO")
            (Actor|DestroyActor _returnvalue_2)
            (bind _returnvalue_3 (Game|SpawnActorfromClass "/Game/PCG/BP_WallDestroyer.BP_WallDestroyer_C" (Math|Transform|MakeTransform (Transformation|GetWorldLocation (Utilities|Array|Get(acopy) (Variables|Default|GetPossibleDoors) (Variables|Default|GetChosen%20Index))) (Math|Rotator|MakeRotator 0.0 0.0 (.yaw (Transformation|GetWorldRotation (Utilities|Array|Get(acopy) (Variables|Default|GetPossibleDoors) (Variables|Default|GetChosen%20Index))))) "1.000000,1.000000,1.000000") "AlwaysSpawn" "MultiplyWithRoot" 0 0))
            (CallFunction|GetRotation (Utilities|Array|Get(acopy) (Variables|Default|GetPossibleDoors) (Variables|Default|GetChosen%20Index)) _returnvalue_3 1e+02 2e+02 -5e+01)
            (bind _returnvalue_4 (Game|SpawnActorfromClass "/Game/PCG/BP_Tunnel.BP_Tunnel_C" (Math|Transform|MakeTransform (Transformation|GetWorldLocation (Utilities|Array|Get(acopy) (Variables|Default|GetPossibleDoors) (Variables|Default|GetChosen%20Index))) (Math|Rotator|MakeRotator 0.0 0.0 (.yaw (Transformation|GetWorldRotation (Utilities|Array|Get(acopy) (Variables|Default|GetPossibleDoors) (Variables|Default|GetChosen%20Index))))) "1.000000,1.000000,1.000000") "AlwaysSpawn" "MultiplyWithRoot" 0 0))
            (PCG|Generate (Variables|/Game/PCG/BP_Tunnel.BP_Tunnel_C|GetPCGTunnel _returnvalue_4) false)
            (Transformation|SetWorldTransform (Variables|/Game/PCG/BP_Tunnel.BP_Tunnel_C|GetExit _returnvalue_4) (Math|Transform|MakeTransform (.location (Transformation|GetWorldTransform (Variables|/Game/PCG/BP_Tunnel.BP_Tunnel_C|GetExit _returnvalue_4))) (.rotation (Transformation|GetWorldTransform (Utilities|Array|Get(acopy) (Variables|Default|GetPossibleDoors) (Variables|Default|GetChosen%20Index)))) (.scale (Transformation|GetWorldTransform (Variables|/Game/PCG/BP_Tunnel.BP_Tunnel_C|GetExit _returnvalue_4)))) false false)
            (Utilities|Array|Add _possibledoors_2 (Variables|/Game/PCG/BP_Tunnel.BP_Tunnel_C|GetExit _returnvalue_4))
            (Utilities|Array|RemoveIndex _possibledoors_2 (Variables|Default|GetChosen%20Index))
            (Development|PrintString "done spawning")
            (CallFunction|GenerateAnotherRoom)))
        (else
          (Utilities|FlowControl|Delay 0.1)
          (goto _label_3)))
      (else
        (Development|PrintString "No exits")))
    (else
      (Utilities|FlowControl|Delay 0.2)
      (goto _label))))

(event EventBeginPlay
  (Math|Random|SetRandomStreamSeed (Variables|Default|GetStream) (Variables|Default|GetRandom%20Seed))
  (CallFunction|GenerateFirstRoom)
  (CallFunction|GenerateTunnel))

(event Collision|EventActorBeginOverlap
  (params (OtherActor :type Actor%20Object%20Reference)))

(event EventTick
  (params (DeltaSeconds :type Float%20%28single-precision%29)))

(fn ConstructionScript)

(fn GetRotation
  (params (Object%20Relative%20to%20Rotation :type Scene%20Component%20Object%20Reference) (Object%20to%20be%20Rotated :type Actor%20Object%20Reference) (Offset%20Relative%20X :type Float%20%28double-precision%29) (Offset%20Relative%20Y :type Float%20%28double-precision%29) (Offset%20Relative%20Z :type Float%20%28double-precision%29))
  (bind _returnvalue (Transformation|GetWorldRotation Object%20Relative%20to%20Rotation))
  (bind _returnvalue_2 (* Offset%20Relative%20X -1.0))
  (bind _returnvalue_3 (* Offset%20Relative%20Y -1.0))
  (if (and (>= (.yaw _returnvalue) -45.0) (<= (.yaw _returnvalue) 45.0))
    (Transformation|AddActorWorldOffset Object%20to%20be%20Rotated (Math|Vector|MakeVector _returnvalue_2 _returnvalue_3 Offset%20Relative%20Z))
    (elif (and (>= (.yaw _returnvalue) 135.0) (<= (.yaw _returnvalue) 225.0))
      (Transformation|AddActorWorldOffset Object%20to%20be%20Rotated (Math|Vector|MakeVector Offset%20Relative%20X Offset%20Relative%20Y Offset%20Relative%20Z))
      (elif (and (>= (.yaw _returnvalue) 45.0) (<= (.yaw _returnvalue) 135.0))
        (Transformation|AddActorWorldOffset Object%20to%20be%20Rotated (Math|Vector|MakeVector Offset%20Relative%20Y _returnvalue_2 Offset%20Relative%20Z))
        (else
          (Transformation|AddActorWorldOffset Object%20to%20be%20Rotated (Math|Vector|MakeVector _returnvalue_3 Offset%20Relative%20X Offset%20Relative%20Z))))))
  (return))